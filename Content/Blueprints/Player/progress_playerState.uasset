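; Player state that tracks player health and handles damage and death.
; On BeginPlay it binds a damage event that, unless the player is invulnerable, subtracts the damage and passes the new health to progress_gameState.
; A health check then destroys player pawn 0 at zero or below, or otherwise grants a brief delay-timed invulnerability window.
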(event Custom|playerDealtDmg_Event
  (params (Bits :type Integer))
  (bind _returnvalue (Game|GetGameState))
  (bind (_asprogress_game_state _bsuccess) (Utilities|Casting|CastToprogress_gameState _returnvalue))
  ;[1 1 1] Health Management
  (if (not (Variables|Default|GetinvulnState))
    (bind _output_get (Variables|Default|SetplayerHealth (- (Variables|Default|GetplayerHealth) Bits)))
    (Default|CallUpdatePlayerHealth _asprogress_game_state _bsuccess _output_get)
    (CallFunction|HealthCheck)))

(event Custom|HealthCheck
  ;[1 1 1] Death Check
  (bind _player_dead (CallFunction|DeathCheck (Variables|Default|GetplayerHealth)))
  (if _player_dead
    (Actor|DestroyActor (Game|Player|GetPlayerPawn 0))
    (else
      (Variables|Default|SetinvulnState true)
      (Utilities|FlowControl|Delay 0.2)
      (Variables|Default|SetinvulnState false))))

(event EventBeginPlay
  ;[1 1 1] Setup
  (EventDispatchers|BindEventtoPlayerDealtDmg (delegate Custom|playerDealtDmg_Event)))

(fn ConstructionScript)

(fn DeathCheck
  (params (playerHealth :type Integer))
  (Math|Integer|CompareInt playerHealth 0
    (:==
      _)
    (:<
      _))
  (bind _output_get (Variables|Default|SetplayerDead true))
  (return _output_get))