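; Actor component that keeps the player inside the visible screen and destroys other owners that leave it.
; Every tick it projects the owner's location to screen space and compares it with the viewport bounds.
; An owner tagged "player" crossing the inset margins is nudged back along world X or Y, one edge per tick, via a location-only transform.
; Any untagged owner outside the viewport is destroyed.
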(event EventTick
  (params (DeltaSeconds :type Float%20%28single-precision%29))
  (bind _returnvalue (Game|GetPlayerController 0))
  (bind _returnvalue_2 (Viewport|GetViewportSize))
  (bind _self self)
  (bind _returnvalue_3 (- (.y _returnvalue_2) 15.0))
  (bind _returnvalue_4 (- (.x _returnvalue_2) 5.0))
  (bind _returnvalue_5 (Components|GetOwner _self))
  (bind _returnvalue_6 (Transformation|GetActorLocation _returnvalue_5))
  (bind (_x _y _z) (Math|Vector|BreakVector _returnvalue_6))
  (bind (_x_2 _y_2 _z_2) (Math|Vector|BreakVector _returnvalue_6))
  (bind _screenlocation (Class|PlayerController|ProjectWorldLocationtoScreen _returnvalue _returnvalue_6 false))
  (bind (_x_3 _y_3 _z_3) (Math|Vector|BreakVector _returnvalue_6))
  (bind (_x_4 _y_4 _z_4) (Math|Vector|BreakVector _returnvalue_6))
  (bind _returnvalue_7 (>= (.y _screenlocation) 15.0))
  (bind _returnvalue_8 (>= (.x _screenlocation) 5.0))
  (bind _returnvalue_9 (<= (.y _screenlocation) _returnvalue_3))
  (bind _returnvalue_10 (<= (.x _screenlocation) _returnvalue_4))
  ;[1 1 1] Offscreen Object Detection
  ;[1 1 1] Player Detection and Boundaries
  (if (Actor|ActorHasTag _returnvalue_5 "player")
    (if (not (Math|Boolean|ANDBoolean _returnvalue_8 _returnvalue_7 _returnvalue_10 _returnvalue_9))
      (if _returnvalue_8
        (if _returnvalue_7
          (if _returnvalue_10
            (if (not _returnvalue_9)
              (Transformation|SetActorTransform _returnvalue_5 (Math|Conversions|ToTransform(Vector) (Math|Vector|MakeVector _x_4 (- _y_4 3e+01) _z_4))))
            (else
              (Transformation|SetActorTransform _returnvalue_5 (Math|Conversions|ToTransform(Vector) (Math|Vector|MakeVector (- _x_3 3e+01) _y_3 _z_3)))))
          (else
            (Transformation|SetActorTransform _returnvalue_5 (Math|Conversions|ToTransform(Vector) (Math|Vector|MakeVector _x (+ _y 3e+01) _z)))))
        (else
          (Transformation|SetActorTransform _returnvalue_5 (Math|Conversions|ToTransform(Vector) (Math|Vector|MakeVector (+ _x_2 3e+01) _y_2 _z_2))))))
    (elif (not (Math|Boolean|ANDBoolean (> (.x _screenlocation) 0.0) (> (.y _screenlocation) 0.0) (< (.x _screenlocation) (.x _returnvalue_2)) (< (.y _screenlocation) (.y _returnvalue_2))))
      (Actor|DestroyActor _returnvalue_5))))