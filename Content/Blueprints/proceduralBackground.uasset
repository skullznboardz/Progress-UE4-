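; Procedural background Blueprint that scrolls three background pieces (large, medium and small) through the level.
; Each Tick, it moves every piece along world Y by BgPieceSpeed times delta seconds, keeping X and Z unchanged.
; All three share one speed, and the file shows no wrapping, respawning or generation logic; the Construction Script is empty.
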(event EventTick
  (params (DeltaSeconds :type Float%20%28single-precision%29))
  (bind _lgpiece (Variables|Default|GetlgPiece))
  (bind _medpiece (Variables|Default|GetmedPiece))
  (bind _smpiece (Variables|Default|GetsmPiece))
  (bind _returnvalue (Transformation|GetWorldTransform _smpiece))
  (bind _returnvalue_2 (Transformation|GetWorldTransform _lgpiece))
  (bind _returnvalue_3 (Transformation|GetWorldTransform _medpiece))
  (bind _location (Math|Transform|BreakTransform _returnvalue))
  (bind _location_2 (Math|Transform|BreakTransform _returnvalue_2))
  (bind _location_3 (Math|Transform|BreakTransform _returnvalue_3))
  (bind (_x _y _z) (Math|Vector|BreakVector _location))
  (bind (_x_2 _y_2 _z_2) (Math|Vector|BreakVector _location_2))
  (bind (_x_3 _y_3 _z_3) (Math|Vector|BreakVector _location_3))
  (Transformation|SetWorldLocation _lgpiece (Math|Vector|MakeVector _x_2 (+ (* (Utilities|Time|GetWorldDeltaSeconds) (Variables|Default|GetbgPieceSpeed)) _y_2) _z_2) false false)
  (Transformation|SetWorldLocation _medpiece (Math|Vector|MakeVector _x_3 (+ (* (Utilities|Time|GetWorldDeltaSeconds) (Variables|Default|GetbgPieceSpeed)) _y_3) _z_3) false false)
  (Transformation|SetWorldLocation _smpiece (Math|Vector|MakeVector _x (+ (* (Utilities|Time|GetWorldDeltaSeconds) (Variables|Default|GetbgPieceSpeed)) _y) _z) false false))

(fn ConstructionScript)