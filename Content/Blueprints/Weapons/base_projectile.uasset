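; Base projectile actor that deals point damage to players and enemies it hits, then destroys itself.
; On a collision component hit, a sequence runs separate enemy and player damage functions, each followed by destroy.
; Each function casts the hit actor to its target class before applying projectile damage with the hit info.
; Only enemy damage passes the instigator's controller as the event instigator.
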(event OnComponentHit(bulletColission)
  (params (HitComponent :type Primitive%20Component%20Object%20Reference) (OtherActor :type Actor%20Object%20Reference) (OtherComp :type Primitive%20Component%20Object%20Reference) (NormalImpulse :type Vector) (Hit :type Hit%20Result%20Structure%20%28by%20ref%29))
  (bind _self self)
  (bind _projectile_damage (Variables|Default|Getprojectile_damage))
  (bind _returnvalue (Math|Conversions|ToFloat(Integer) _projectile_damage))
  ;[1 1 1] Projectile Damage
  (Utilities|FlowControl|Sequence
    (:then_0
      (CallFunction|DamageEnemy OtherActor _returnvalue NormalImpulse Hit _self))
    (:then_1
      (CallFunction|DamagePlayer OtherActor _returnvalue NormalImpulse Hit _self)))
  (Actor|DestroyActor))

(fn ConstructionScript)

(fn DamagePlayer
  (params (Object :type Object%20Object%20Reference) (BaseDamage :type Float%20%28single-precision%29) (HitFromDirection :type Vector%20%28by%20ref%29) (HitInfo :type Hit%20Result%20Structure%20%28by%20ref%29) (DamageCauser :type Actor%20Object%20Reference))
  (bind _asprogress_pawn (Utilities|Casting|CastToprogress_pawn Object))
  (Game|Damage|ApplyPointDamage _asprogress_pawn BaseDamage HitFromDirection HitInfo 0 DamageCauser))

(fn DamageEnemy
  (params (Object :type Object%20Object%20Reference) (BaseDamage :type Float%20%28single-precision%29) (HitFromDirection :type Vector%20%28by%20ref%29) (HitInfo :type Hit%20Result%20Structure%20%28by%20ref%29) (DamageCauser :type Actor%20Object%20Reference))
  (bind _asbase_enemy (Utilities|Casting|CastTobase_enemy Object))
  (Game|Damage|ApplyPointDamage _asbase_enemy BaseDamage HitFromDirection HitInfo (Pawn|GetController (Variables|Actor|GetInstigator)) DamageCauser))